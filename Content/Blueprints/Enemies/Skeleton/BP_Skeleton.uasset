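; Skeleton enemy for a side-view sprite game that patrols back and forth along X and damages BP_Hero on contact.
; Tick runs Follow, which counts frames toward a signed limit, then flips direction and sprite rather than tracking the hero.
; BoxHit overlap applies damage, passes its X to the hero and briefly pauses movement.
; Taking damage launches it away from the hero and destroys it when Health runs out.
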(event OnComponentBeginOverlap(BoxHit)
  (params (OverlappedComponent :type Primitive%20Component%20Object%20Reference) (OtherActor :type Actor%20Object%20Reference) (OtherComp :type Primitive%20Component%20Object%20Reference) (OtherBodyIndex :type Integer) (bFromSweep :type Boolean) (SweepResult :type Hit%20Result%20Structure%20%28by%20ref%29))
  (bind _returnvalue (Components|GetOwner))
  (Utilities|IsValid _returnvalue
    (:Is%20Valid
      (if (not (== _returnvalue OtherActor))
        (bind _asbp_hero (Utilities|Casting|CastToBP_Hero OtherActor))
        (Game|Damage|ApplyDamage _asbp_hero 15.0 0 0)
        (Variables|/Game/Blueprints/Hero/BP_Hero.BP_Hero_C|SetEnemyPosX (Variables|Default|GetBP%20Hero) (.x (Transformation|GetWorldLocation (Variables|Default|GetSprite))))
        (Variables|Default|SetisMovementLock true)
        (Utilities|FlowControl|Delay 0.4)
        (Variables|Default|SetisMovementLock false)))))

(event Custom|Follow
  (if (not (Variables|Default|GetisMovementLock))
    (Math|Float|CompareFloat (Variables|Default|Gets1) (Variables|Default|Gets)
      (:>
        (Pawn|Input|AddMovementInput "-1.000000,0.000000,0.000000" 1.0 false)
        (Variables|Default|Sets1 (- (Variables|Default|Gets1) 1.0)))
      (:==
        (if (> (Variables|Default|Gets) 0.0)
          (Variables|Default|Sets (* (Variables|Default|Gets) -1.0))
          (Variables|Default|Sets1 0.0)
          (Transformation|SetRelativeRotation (Variables|Default|GetSprite) "0.000000,180.000000,0.000000" false false)
          (else
            (Variables|Default|Sets (* (Variables|Default|Gets) -1.0))
            (Variables|Default|Sets1 0.0)
            (Transformation|SetRelativeRotation (Variables|Default|GetSprite) "0, 0, 0" false false))))
      (:<
        (Pawn|Input|AddMovementInput "1.000000,0.000000,0.000000" 1.0 false)
        (Variables|Default|Sets1 (+ (Variables|Default|Gets1) 1.0))))))

(event EventBeginPlay
  (bind _asbp_hero (Utilities|Casting|CastToBP_Hero (Game|GetPlayerCharacter 0)))
  (Variables|Default|SetBP%20Hero _asbp_hero))

(event Collision|EventActorBeginOverlap
  (params (OtherActor :type Actor%20Object%20Reference)))

(event EventTick
  (params (DeltaSeconds :type Float%20%28single-precision%29))
  (CallFunction|Follow))

(event Game|Damage|EventAnyDamage
  (params (Damage :type Float%20%28single-precision%29) (DamageType :type Damage%20Type%20Object%20Reference) (InstigatedBy :type Controller%20Object%20Reference) (DamageCauser :type Actor%20Object%20Reference))
  (if (not (Variables|Default|GetisDead))
    (Math|Float|CompareFloat (.x (Transformation|GetWorldLocation (Variables|/Script/Paper2D.PaperCharacter|GetSprite (Variables|Default|GetBP%20Hero)))) (.x (Transformation|GetWorldLocation (Variables|Default|GetSprite)))
      (:>
        (Character|LaunchCharacter "-800.000000,0.000000,100.000000" true true))
      (:<
        (Character|LaunchCharacter "800.000000,0.000000,100.000000" true true)))
    (Variables|Default|SetHealth (- (Variables|Default|GetHealth) Damage))
    (Development|PrintString (Utilities|String|Append "Skeleton's Health: " (Utilities|String|ToString(Float) (Variables|Default|GetHealth))))
    (if (> (Variables|Default|GetHealth) 0.0)
      (Variables|Default|SetisMovementLock true)
      (Utilities|FlowControl|Delay 0.0)
      (Variables|Default|SetisMovementLock false)
      (else
        (Variables|Default|SetisMovementLock true)
        (Variables|Default|SetisDead true)
        (Actor|DestroyActor)))))

(fn ConstructionScript)