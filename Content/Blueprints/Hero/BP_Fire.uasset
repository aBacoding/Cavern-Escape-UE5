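; BP_Fire is a magic attack projectile, filed under Hero, that damages what it hits.
; When its Box overlaps another actor, it plays a sonic hit sound and applies fixed damage.
; It then hides the projectile visual, halts ProjectileMovement, shows a one-shot Hit effect and destroys itself after a short delay.
; The only overlap filter excludes itself, with no check against the shooter.
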(event OnComponentBeginOverlap(Box)
  (params (OverlappedComponent :type Primitive%20Component%20Object%20Reference) (OtherActor :type Actor%20Object%20Reference) (OtherComp :type Primitive%20Component%20Object%20Reference) (OtherBodyIndex :type Integer) (bFromSweep :type Boolean) (SweepResult :type Hit%20Result%20Structure%20%28by%20ref%29))
  (bind _projectilemovement (Variables|Default|GetProjectileMovement))
  (bind _hit (Variables|Default|GetHit))
  ;[1 1 1] Magic Attack System
  (if (!= OtherActor self)
    (Audio|PlaySound2D "/Game/Assets/Fire/Sounds/Sonic_Pulse_Hit_02.Sonic_Pulse_Hit_02" 1.0 1.0 0.0 0 0)
    (Game|Damage|ApplyDamage OtherActor 25.0 0 0)
    (Rendering|SetVisibility (Variables|Default|GetProjectTile) false false)
    (Variables|/Script/Engine.ProjectileMovementComponent|SetProjectileGravityScale _projectilemovement 0.0)
    (Components|Movement|StopMovementImmediately _projectilemovement)
    (Rendering|SetVisibility _hit true false)
    (Components|Timeline|SetPlayRate _hit 1.0)
    (Components|Timeline|SetLooping _hit false)
    (Utilities|FlowControl|Delay 0.35)
    (Actor|DestroyActor)))

(event EventBeginPlay)

(event Collision|EventActorBeginOverlap
  (params (OtherActor :type Actor%20Object%20Reference)))

(event EventTick
  (params (DeltaSeconds :type Float%20%28single-precision%29)))

(fn ConstructionScript)