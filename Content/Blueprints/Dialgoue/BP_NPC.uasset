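; BP_NPC is an interactable NPC that steps through dialogue lines and ends the level once they run out.
; A trigger shows its prompt widget while BP_Hero overlaps it.
; Each Interact increments DialogueIndex and writes that array entry to a WB_Dialogue widget, created if not already valid.
; When the index reaches the array length, it adds WB_Level_Complete, pauses the game and removes the dialogue widget.
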(event OnComponentBeginOverlap(Trigger)
  (params (OverlappedComponent :type Primitive%20Component%20Object%20Reference) (OtherActor :type Actor%20Object%20Reference) (OtherComp :type Primitive%20Component%20Object%20Reference) (OtherBodyIndex :type Integer) (bFromSweep :type Boolean) (SweepResult :type Hit%20Result%20Structure%20%28by%20ref%29))
  ;[1 1 1] Show the interaction prompt
  (Utilities|Casting|CastToBP_Hero OtherActor)
  (Rendering|SetVisibility (Variables|Default|GetwidgetPrompt) true false))

(event OnComponentEndOverlap(Trigger)
  (params (OverlappedComponent :type Primitive%20Component%20Object%20Reference) (OtherActor :type Actor%20Object%20Reference) (OtherComp :type Primitive%20Component%20Object%20Reference) (OtherBodyIndex :type Integer))
  ;[1 1 1] Do not show the interaction prompt
  (Utilities|Casting|CastToBP_Hero OtherActor)
  (Rendering|SetVisibility (Variables|Default|GetwidgetPrompt) false false))

(event EventBeginPlay)

(event Collision|EventActorBeginOverlap
  (params (OtherActor :type Actor%20Object%20Reference)))

(event EventTick
  (params (DeltaSeconds :type Float%20%28single-precision%29)))

(event EventInteract
  (Math|Integer|IncrementInt (Variables|Default|GetDialogueIndex)
    (:%20%20
      (if (<= (Variables|Default|GetDialogueIndex) (Utilities|Array|Length (Variables|Default|GetDialogue)))
        (Variables|Default|GetUI
          (:then
            _)
          (:else
            (bind _returnvalue (UserInterface|CreateWidget "/Game/Blueprints/Dialgoue/WB_Dialogue.WB_Dialogue_C" (Game|GetPlayerController 0)))
            (bind _output_get (Variables|Default|SetUI _returnvalue))
            (UserInterface|Viewport|AddtoViewport _output_get 0)))
        (Rendering|Components|TextRender|SetText (Variables|/Game/Blueprints/Dialgoue/WB_Dialogue.WB_Dialogue_C|GetDialogueText (Variables|Default|GetUI)) (Utilities|Text|ToText(String) (Utilities|Array|Get(acopy) (Variables|Default|GetDialogue) (Variables|Default|GetDialogueIndex))))
        (if (>= (Variables|Default|GetDialogueIndex) (Utilities|Array|Length (Variables|Default|GetDialogue)))
          (bind _returnvalue_2 (UserInterface|CreateWidget "/Game/UI/Menu/WB_Level_Complete.WB_Level_Complete_C"))
          (UserInterface|Viewport|AddtoViewport _returnvalue_2 0)
          (Game|SetGamePaused true)
          (Widget|RemovefromParent (Variables|Default|GetUI)))))))

(fn ConstructionScript
  (Rendering|SetVisibility (Variables|Default|GetwidgetPrompt) false false))